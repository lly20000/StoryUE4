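; Story dialogue player that shows visual-novel style conversations in a StoryUI widget, created hidden at BeginPlay.
; It caches a fixed count of DataTable rows, then Tick uses a Delay as a throttle to type the current line character by character at a selectable speed.
; Each row sets speaker name, left/right portrait with the other side dimmed, and background.
; Events toggle playback and advance via each row's NextItem; rows outside the current Section hide the UI.
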(event Custom|LoadStoryData
  (params (ItemCount :type Integer))
  ;[1 1 1] 加载文字数据
  (bind _output_get (Variables|Default|SetDataTable "/Game/Story/DataBase/StoryText.StoryText"))
  (while (< (Variables|Default|GetItemIndex) ItemCount)
    (bind _returnvalue (Utilities|GetDataTableRow _output_get (Utilities|String|StringToName (Utilities|String|ToString(Integer) (Variables|Default|GetItemIndex))))
      (:then
        (CallFunction|AddStoryTextSource _returnvalue)
        (bind _result (Math|Integer|IncrementInt (Variables|Default|GetItemIndex))
          (:%20%20
            (Variables|Default|SetItemIndex _result)))))))

(event Custom|LoadUI
  ;[1 1 1] 添加UI
  (bind _returnvalue (UserInterface|CreateWidget "/Game/Story/UI/StoryUI.StoryUI_C"))
  (UserInterface|Viewport|AddtoViewport _returnvalue 0)
  (bind _output_get (Variables|Default|SetStoryUI _returnvalue))
  (Default|UpdateSection _output_get 1)
  (Variables|Default|SetPlayStory false)
  (Widget|SetVisibility (Variables|Default|GetStoryUI) "Hidden"))

(event Custom|OpenStoryTextPlay
  (params (PlayStory :type Boolean))
  (if PlayStory
    (Variables|Default|SetPlayStory true)
    (Widget|SetVisibility (Variables|Default|GetStoryUI) "Visible")
    (else
      (Variables|Default|SetPlayStory false)
      (Widget|SetVisibility (Variables|Default|GetStoryUI) "Hidden"))))

(event Custom|UpdateStorySourceIndex
  (params (StoryIndex :type Integer))
  (Variables|Default|SetStoryTextSourceIndex StoryIndex))

(event Custom|ClearStoryText
  ;[1 1 1] 清除对话框文字
  (bind _output_get (Variables|Default|SetStoryText ""))
  (Variables|Default|SetStoryTextIndex 0)
  (Rendering|Components|TextRender|SetText (Variables|/Game/Story/UI/StoryUI.StoryUI_C|GetRichTextBlock_Story (Variables|Default|GetStoryUI)) (Utilities|Text|ToText(String) _output_get)))

(event Custom|AddStoryTextSource
  (params (StoryItem :type Story%20Struct%20Structure))
  ;[1 1 1] 添加原始数据表
  (Utilities|Array|Add (Variables|Default|GetStoryTextSource) StoryItem))

(event Custom|CookStoryText
  (bind _storytextsourceindex (Variables|Default|GetStoryTextSourceIndex))
  (bind _storytextsource (Variables|Default|GetStoryTextSource))
  (bind _returnvalue (Utilities|Array|Length _storytextsource))
  (bind _output (Utilities|Array|Get(acopy) _storytextsource _storytextsourceindex))
  (bind (_speaker _background _text _scene _audio _music _section _speakerleftright _speakerimage _nextitem) (Utilities|Struct|BreakStoryStruct _output))
  (bind _returnvalue_2 (Utilities|String|Len _text))
  ;[1 1 1] 打字机效果
  (if (Variables|Default|GetPlayStory)
    (if (>= (Variables|Default|GetStoryTextSourceIndex) 0)
      (if (> _returnvalue 0)
        (if (and (>= _storytextsourceindex 0) (> _returnvalue 0))
          (Utilities|FlowControl|Delay (Variables|Default|GetWaittime))
          (if (== _section (Variables|Default|GetSection))
            (if (> _returnvalue_2 0)
              (if (< (Variables|Default|GetStoryTextIndex) _returnvalue_2)
                (Development|PrintString _text)
                (CallFunction|UpdateSpeaker _speaker _speakerleftright)
                (CallFunction|UpdatePersonImage _speakerimage _speakerleftright)
                (CallFunction|UpdateBackground _background)
                (bind _output_get (Variables|Default|SetStoryText (Utilities|String|Append (Variables|Default|GetStoryText) (Utilities|String|GetSubstring _text (Variables|Default|GetStoryTextIndex)))))
                (Rendering|Components|TextRender|SetText (Variables|/Game/Story/UI/StoryUI.StoryUI_C|GetRichTextBlock_Story (Variables|Default|GetStoryUI)) (Utilities|Text|ToText(String) _output_get))
                (bind _result (Math|Integer|IncrementInt (Variables|Default|GetStoryTextIndex))
                  (:%20%20
                    (Variables|Default|SetStoryTextIndex _result)
                    (Variables|Default|SetNextStoryTextSourceIndex _nextitem)))))
            (else
              (Widget|SetVisibility (Variables|Default|GetStoryUI) "Hidden"))))))))

(event Custom|ResetNextStoryText
  ;[1 1 1] 开始下一段的文字内容
  (if (Variables|Default|GetPlayStory)
    (CallFunction|ClearStoryText)
    (Variables|Default|SetStoryTextSourceIndex (Variables|Default|GetNextStoryTextSourceIndex))))

(event Custom|UpdatePlaySpeed
  (params (SpeedLvl :type Integer))
  ;[1 1 1] 更新文字刷新速度
  (switch int SpeedLvl
    (:Default
      (Variables|Default|SetWaittime 0.2))
    (:0
      (Variables|Default|SetWaittime 0.2))
    (:1
      (Variables|Default|SetWaittime 0.1))
    (:2
      (Variables|Default|SetWaittime 0.05))))

(event Custom|UpdateSpeaker
  (params (Speaker :type String) (Left :type Integer))
  (bind _returnvalue (Utilities|Text|ToText(String) Speaker))
  ;[1 1 1] 更新Speaker的名称
  (switch int Left
    (:Default
      (Rendering|Components|TextRender|SetText (Variables|/Game/Story/UI/StoryUI.StoryUI_C|GetTextBlock_SpeakerLeft (Variables|Default|GetStoryUI)) _returnvalue :!label _label))
    (:0
      (goto _label))
    (:1
      (goto _label))
    (:2
      (Rendering|Components|TextRender|SetText (Variables|/Game/Story/UI/StoryUI.StoryUI_C|GetTextBlock_SpeakerRight (Variables|Default|GetStoryUI)) _returnvalue))))

(event Custom|UpdatePersonImage
  (params (Imagename :type String) (LeftOrRigh :type Integer))
  (bind _returnvalue (- LeftOrRigh 1))
  (bind _imagedata (Variables|Default|GetImageData))
  (bind _output (Utilities|Array|Get(acopy) _imagedata _returnvalue))
  (bind _returnvalue_2 (Utilities|Enum|NotEqual(Enum) Imagename _output))
  ;[1 1 1] 更新配置的对话图像
  (if (and (Utilities|Enum|NotEqual(Enum) Imagename "None") (> (Utilities|String|Len Imagename) 0))
    (switch int _returnvalue
      (:0
        (if _returnvalue_2
          (bind _returnvalue_3 (Class|ResourceManagerAPI|LoadContentTexture Imagename))
          (Widget|SetVisibility (Variables|/Game/Story/UI/StoryUI.StoryUI_C|GetImage_Left (Variables|Default|GetStoryUI)) "Visible")
          (Appearance|SetBrushfromTexture (Variables|/Game/Story/UI/StoryUI.StoryUI_C|GetImage_Left (Variables|Default|GetStoryUI)) _returnvalue_3 false)
          (Class|Image|SetBrushTintColor (Variables|/Game/Story/UI/StoryUI.StoryUI_C|GetImage_Left (Variables|Default|GetStoryUI)) (Utilities|Struct|MakeSlateColor "(R=1.000000,G=1.000000,B=1.000000,A=1.000000)" "UseColor_Specified"))
          (Class|Image|SetBrushTintColor (Variables|/Game/Story/UI/StoryUI.StoryUI_C|GetImage_Right (Variables|Default|GetStoryUI)) (Utilities|Struct|MakeSlateColor "(R=0.333333,G=0.333333,B=0.333333,A=1.000000)" "UseColor_Specified"))))
      (:1
        (if _returnvalue_2
          (bind _returnvalue_4 (Class|ResourceManagerAPI|LoadContentTexture Imagename))
          (Widget|SetVisibility (Variables|/Game/Story/UI/StoryUI.StoryUI_C|GetImage_Right (Variables|Default|GetStoryUI)) "Visible")
          (Appearance|SetBrushfromTexture (Variables|/Game/Story/UI/StoryUI.StoryUI_C|GetImage_Right (Variables|Default|GetStoryUI)) _returnvalue_4 false)
          (Class|Image|SetBrushTintColor (Variables|/Game/Story/UI/StoryUI.StoryUI_C|GetImage_Left (Variables|Default|GetStoryUI)) (Utilities|Struct|MakeSlateColor "(R=0.333333,G=0.333333,B=0.333333,A=1.000000)" "UseColor_Specified"))
          (Class|Image|SetBrushTintColor (Variables|/Game/Story/UI/StoryUI.StoryUI_C|GetImage_Right (Variables|Default|GetStoryUI)) (Utilities|Struct|MakeSlateColor "(R=1.000000,G=1.000000,B=1.000000,A=1.000000)" "UseColor_Specified")))))))

(event Custom|UpdateBackground
  (params (bkname :type String))
  (if (Utilities|Enum|Equal(Enum) bkname "None")
    (Widget|SetVisibility (Variables|/Game/Story/UI/StoryUI.StoryUI_C|GetImage_BK (Variables|Default|GetStoryUI)) "Hidden")
    (else
      (Widget|SetVisibility (Variables|/Game/Story/UI/StoryUI.StoryUI_C|GetImage_BK (Variables|Default|GetStoryUI)) "Visible")
      (if (Utilities|Enum|NotEqual(Enum) (Variables|Default|GetBkImageName) bkname)
        (bind _returnvalue (Class|ResourceManagerAPI|LoadContentTexture bkname))
        (Appearance|SetBrushfromTexture (Variables|/Game/Story/UI/StoryUI.StoryUI_C|GetImage_BK (Variables|Default|GetStoryUI)) _returnvalue false)
        (Variables|Default|SetBkImageName (Variables|Default|GetBkImageName))))))

(event EventBeginPlay
  (CallFunction|LoadUI)
  (CallFunction|LoadStoryData 19))

(event Collision|EventActorBeginOverlap
  (params (OtherActor :type Actor%20Object%20Reference)))

(event EventTick
  (params (DeltaSeconds :type Float%20%28single-precision%29))
  (CallFunction|CookStoryText))

(fn ConstructionScript)