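; StoryActive_BP is an interaction actor that starts story text playback when the player presses a key nearby.
; Begin and end overlap with ThirdPersonCharacter toggle the CookInput flag, which gates the ActionPress input.
; On a valid press it finds the Story_BP actor by class, calls OpenStoryTextPlay, then resets the story source index to the hard-coded first entry.
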(event EventBeginPlay)

(event Collision|EventActorBeginOverlap
  (params (OtherActor :type Actor%20Object%20Reference))
  (bind _asthird_person_character (Utilities|Casting|CastToThirdPersonCharacter OtherActor))
  (if (Utilities|IsValid _asthird_person_character)
    (Variables|Default|SetCookInput true)))

(event EventTick
  (params (DeltaSeconds :type Float%20%28single-precision%29)))

(event Collision|EventActorEndOverlap
  (params (OtherActor :type Actor%20Object%20Reference))
  (bind _asthird_person_character (Utilities|Casting|CastToThirdPersonCharacter OtherActor))
  (if (Utilities|IsValid _asthird_person_character)
    (Variables|Default|SetCookInput false)))

(event Input|ActionEvents|InputActionActionPress
  (params (Key :type Key%20Structure :default "None"))
  (:Pressed
    (if (Variables|Default|GetCookInput)
      (bind _returnvalue (Actor|GetActorOfClass "/Game/Story/Blueprint/Story_BP.Story_BP_C"))
      (Default|OpenStoryTextPlay _returnvalue true)
      (Default|UpdateStorySourceIndex _returnvalue))))

(fn ConstructionScript)